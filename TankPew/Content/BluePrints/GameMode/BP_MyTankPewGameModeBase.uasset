(event EventBeginPlay)

(event EventStartGame
  (bind _returnvalue (UserInterface|CreateWidget "/Game/BluePrints/Widgets/WBP_StartGameWidget.WBP_StartGameWidget_C"))
  (UserInterface|Viewport|AddtoViewport _returnvalue 0))

(event EventGameOver
  (params (aWonGame :type Boolean))
  (bind _returnvalue (UserInterface|CreateWidget "/Game/BluePrints/Widgets/WBP_GameOverWidget.WBP_GameOverWidget_C"))
  (UserInterface|Viewport|AddtoViewport _returnvalue 0)
  (Rendering|Components|TextRender|SetText (Variables|/Game/BluePrints/Widgets/WBP_GameOverWidget.WBP_GameOverWidget_C|GetDisplayText _returnvalue) (select aWonGame "You Won!" "Game Over!")))

(event EventTick
  (params (DeltaSeconds :type Float%20%28single-precision%29))
  (bind _returnvalue (UserInterface|CreateWidget "/Game/BluePrints/Widgets/WBP_MainGameWidget.WBP_MainGameWidget_C"))
  (UserInterface|Viewport|AddtoViewport _returnvalue 0))

(fn ConstructionScript)